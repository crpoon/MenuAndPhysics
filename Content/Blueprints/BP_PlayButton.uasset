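; BP_PlayButton is a menu play button that loads the PhysicsPlayground level when selected.
; Select has the BP_MenuPlayer pawn fade to black, waits briefly, then opens the level by name.
; HoverOn and HoverOff switch the TextRender color between blue and white as highlight feedback.
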(event Custom|Select
  (bind _asbp_menu_player (Utilities|Casting|CastToBP_MenuPlayer (Game|Player|GetPlayerPawn 0)))
  (Default|FadetoBlack _asbp_menu_player)
  (Utilities|FlowControl|Delay 1.0)
  (Game|OpenLevel(byName) "PhysicsPlayground"))

(event Custom|HoverOn
  (Rendering|Components|TextRender|SetTextRenderColor (Variables|Default|GetTextRender) (Math|Color|MakeColor 1 0 0 1)))

(event Custom|HoverOff
  (Rendering|Components|TextRender|SetTextRenderColor (Variables|Default|GetTextRender) (Math|Color|MakeColor 1 1 1 1)))

(event EventBeginPlay)

(event EventActorBeginOverlap
  (params (OtherActor :type Actor%20Object%20Reference)))

(event EventTick
  (params (DeltaSeconds :type Float%20%28single-precision%29)))

(fn ConstructionScript)