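; BP_ToggleMusic is an actor that acts as an in-world on/off switch for the BuyAndSell music.
; It starts the track on BeginPlay, and an overlap or hit on its StaticMesh stops it if playing or restarts it from the beginning otherwise.
; Each change is recorded in the IsMusicOn flag on BP_GameInstance through SetMusicOn.
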(event OnComponentBeginOverlap(StaticMesh)
  (params (OtherActor :type Actor%20Object%20Reference) (OtherComp :type Primitive%20Component%20Object%20Reference) (OtherBodyIndex :type Integer) (bFromSweep :type Boolean) (SweepResult :type Hit%20Result%20Structure%20%28by%20ref%29))
  (bind _buyandsell (Variables|Default|GetBuyAndSell))
  (if (Audio|Components|Audio|IsPlaying _buyandsell)
    (Audio|Components|Audio|Stop _buyandsell)
    (CallFunction|SetMusicon false)
    (else
      (Audio|Components|Audio|Play _buyandsell 0.0)
      (CallFunction|SetMusicon true))))

(event OnComponentHit(StaticMesh)
  (params (OtherActor :type Actor%20Object%20Reference) (OtherComp :type Primitive%20Component%20Object%20Reference) (NormalImpulse :type Vector :default "0, 0, 0") (Hit :type Hit%20Result%20Structure%20%28by%20ref%29))
  (bind _buyandsell (Variables|Default|GetBuyAndSell))
  (if (Audio|Components|Audio|IsPlaying _buyandsell)
    (Audio|Components|Audio|Stop _buyandsell)
    (CallFunction|SetMusicon false)
    (else
      (Audio|Components|Audio|Play _buyandsell 0.0)
      (CallFunction|SetMusicon true))))

(event EventBeginPlay
  (Audio|Components|Audio|Play (Variables|Default|GetBuyAndSell) 0.0)
  (CallFunction|SetMusicon true))

(event EventActorBeginOverlap
  (params (OtherActor :type Actor%20Object%20Reference)))

(event EventTick
  (params (DeltaSeconds :type Float%20%28single-precision%29)))

(fn ConstructionScript)

(fn SetMusicon
  (params (IsMusicOn :type Boolean))
  (bind _asbp_game_instance (Utilities|Casting|CastToBP_GameInstance (Game|GetGameInstance))
    (:then
      (Variables|/Game/Blueprints/BP_GameInstance.BP_GameInstance_C|SetIsMusicOn _asbp_game_instance IsMusicOn))
    (:CastFailed
      _))
  (return))