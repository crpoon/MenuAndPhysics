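; BP_ForceText is a text display actor that shows and adjusts an impulse force value stored in BP_GameInstance.
; BeginPlay resets the impulse to a default and writes it to the TextRender.
; LowerForce and AddForce step the value down or up by a fixed amount, with a floor only on lowering, then refresh the text.
; Get and Set helper functions cast the game instance to read and write the shared value.
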(event Custom|Lower%20Force
  (bind _impulse (CallFunction|GetImpulse))
  (if (not (< _impulse 20000))
    (CallFunction|SetImpulse (- _impulse 10000))
    (Rendering|Components|TextRender|SetText (Variables|Default|GetTextRender) (Utilities|Text|ToText(String) (Utilities|String|BuildString(Integer) "" "Impulse: " (- _impulse 10000))))))

(event Custom|Add%20Force
  (bind _impulse (CallFunction|GetImpulse))
  (CallFunction|SetImpulse (+ _impulse 10000))
  (Rendering|Components|TextRender|SetText (Variables|Default|GetTextRender) (Utilities|Text|ToText(String) (Utilities|String|BuildString(Integer) "" "Impulse: " (+ _impulse 10000)))))

(event EventBeginPlay
  (CallFunction|SetImpulse 100000)
  (bind _impulse (CallFunction|GetImpulse))
  (Rendering|Components|TextRender|SetText (Variables|Default|GetTextRender) (Utilities|Text|ToText(String) (Utilities|String|BuildString(Integer) "" "Impulse: " _impulse))))

(fn ConstructionScript)

(fn GetImpulse
  (bind _asbp_game_instance (Utilities|Casting|CastToBP_GameInstance (Game|GetGameInstance))
    (:then
      _)
    (:CastFailed
      _))
  (return (Variables|/Game/Blueprints/BP_GameInstance.BP_GameInstance_C|GetImpulse _asbp_game_instance)))

(fn SetImpulse
  (params (Impulse :type Integer))
  (bind _asbp_game_instance (Utilities|Casting|CastToBP_GameInstance (Game|GetGameInstance))
    (:then
      (Variables|/Game/Blueprints/BP_GameInstance.BP_GameInstance_C|SetImpulse _asbp_game_instance Impulse))
    (:CastFailed
      _))
  (return))